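; Paddles actor for a Pong-style game, driving a left and a right paddle with vertical movement.
; Player 1 and Player 2 axis inputs offset their paddles along Z, scaled by Speed and without sweep.
; Until Player 2 first gives non-zero input, Tick runs the right paddle as AI, easing its height toward the Ball with a per-frame Lerp.
; That first input sets Is2Player, permanently handing over control.
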(event EventTick
  (params (DeltaSeconds :type Float%20%28single-precision%29))
  (bind _right_paddle (Variables|Default|GetRight%20Paddle))
  (if (not (Variables|Default|GetIs%202%20Player))
    (Transformation|SetWorldLocation _right_paddle (Math|Vector|MakeVector 0.0 2e+02 (Math|Float|Lerp (.Z (Math|Vector|BreakVector (Transformation|GetActorLocation (Variables|Default|GetBall)))) (.Z (Math|Vector|BreakVector (Transformation|GetWorldLocation _right_paddle))) 0.985)) false false)))

(event Input|AxisEvents|InputAxisPlayer1
  (params (AxisValue :type Float%20%28single-precision%29))
  (Transformation|AddLocalOffset (Variables|Default|GetLeft%20Paddle) (* (Math|Vector|MakeVector 0.0 0.0 AxisValue) (Variables|Default|GetSpeed)) false false))

(event Input|AxisEvents|InputAxisPlayer2
  (params (AxisValue :type Float%20%28single-precision%29))
  (Math|Float|CompareFloat AxisValue 0.0
    (:>
      _)
    (:<
      _))
  (Variables|Default|SetIs%202%20Player true)
  (Transformation|AddLocalOffset (Variables|Default|GetRight%20Paddle) (* (Math|Vector|MakeVector 0.0 0.0 AxisValue) (Variables|Default|GetSpeed)) false false))

(fn ConstructionScript)