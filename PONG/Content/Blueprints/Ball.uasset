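; Pong-style ball actor driven by a ProjectileMovement component in the Y-Z plane.
; On hitting the Paddles actor at negative Y, it compares its height to LeftPaddle and sets a fixed upward or downward Z velocity; positive-Y hits are not handled.
; Each projectile bounce negates the Y velocity.
; Both handlers feed world velocity into SetVelocityInLocalSpace.
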(event OnProjectileBounce(ProjectileMovement)
  (params (ImpactResult :type Hit%20Result%20Structure%20%28by%20ref%29) (ImpactVelocity :type Vector%20%28by%20ref%29 :default "0, 0, 0"))
  (bind _returnvalue (Transformation|GetVelocity))
  (bind (_x _y _z) (Math|Vector|BreakVector _returnvalue))
  (Game|Components|ProjectileMovement|SetVelocityinLocalSpace (Variables|Default|GetProjectileMovement) (Math|Vector|MakeVector _x (* -1.0 _y) _z)))

(event Collision|EventHit
  (params (MyComp :type Primitive%20Component%20Object%20Reference) (Other :type Actor%20Object%20Reference) (OtherComp :type Primitive%20Component%20Object%20Reference) (bSelfMoved :type Boolean) (HitLocation :type Vector :default "0, 0, 0") (HitNormal :type Vector :default "0, 0, 0") (NormalImpulse :type Vector :default "0, 0, 0") (Hit :type Hit%20Result%20Structure%20%28by%20ref%29))
  (bind _returnvalue (Transformation|GetVelocity))
  (bind _returnvalue_2 (Transformation|GetVelocity))
  (bind _ball (Variables|Default|GetBall))
  (bind _returnvalue_3 (Transformation|GetWorldLocation _ball))
  (bind (_x _y) (Math|Vector|BreakVector _returnvalue))
  (bind (_x_2 _y_2) (Math|Vector|BreakVector _returnvalue_2))
  (bind (_x_3 _y_3 _z) (Math|Vector|BreakVector _returnvalue_3))
  (bind _aspaddles (Utilities|Casting|CastToPaddles Other))
  (Math|Float|CompareFloat _y_3 0.0
    (:<
      (Math|Float|CompareFloat _z (.Z (Math|Vector|BreakVector (Transformation|GetWorldLocation (Variables|/Game/Blueprints/Paddles.Paddles_C|GetLeft%20Paddle _aspaddles))))
        (:>
          (Game|Components|ProjectileMovement|SetVelocityinLocalSpace (Variables|Default|GetProjectileMovement) (Math|Vector|MakeVector _x _y 5e+01)))
        (:<
          (Game|Components|ProjectileMovement|SetVelocityinLocalSpace (Variables|Default|GetProjectileMovement) (Math|Vector|MakeVector _x_2 _y_2 -5e+01)))))))

(fn ConstructionScript)