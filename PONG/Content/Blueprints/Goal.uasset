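; Goal actor that scores when a Ball enters it and shows its own score.
; On overlap it moves the Ball to the world origin, increments Score and writes the new value to ScoreDisplay.
; The Construction Script offsets ScoreDisplay along local Y according to the sign of the goal's world Y, so one Blueprint serves goals on either side of the origin.
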(event Collision|EventActorBeginOverlap
  (params (OtherActor :type Actor%20Object%20Reference))
  (bind _asball (Utilities|Casting|CastToBall OtherActor))
  (Transformation|SetActorLocation _asball "0, 0, 0" false false)
  (bind _result (Math|Integer|IncrementInt (Variables|Default|GetScore))
    (:%20%20
      (Rendering|Components|TextRender|SetText (Variables|Default|GetScoreDisplay) (Utilities|Text|ToText(Integer) _result)))))

(fn ConstructionScript
  (bind _scoredisplay (Variables|Default|GetScoreDisplay))
  (Math|Float|CompareFloat (.Y (Math|Vector|BreakVector (Transformation|GetWorldLocation (Variables|Default|GetDefaultSceneRoot)))) 0.0
    (:>
      (Transformation|SetRelativeLocation _scoredisplay "0,-420.000000,60.000000" false false))
    (:<
      (Transformation|SetRelativeLocation _scoredisplay "0,395.000000,60.000000" false false))))